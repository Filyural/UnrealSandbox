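; Actor component that moves its owner back and forth along its forward vector.
; Tick offsets the owner's location each frame by the forward vector scaled by delta time and DirectionMultiplier, without sweeping for collision.
; A looping Delay started on BeginPlay negates DirectionMultiplier every few seconds to reverse the travel direction.
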(event EventBeginPlay
  (Utilities|FlowControl|Delay 4.0 :!label _label)
  (Variables|Default|SetDirectionMultiplier (* (Variables|Default|GetDirectionMultiplier) -1))
  (goto _label))

(event EventTick
  (params (DeltaSeconds :type Float%20%28single-precision%29))
  (bind _returnvalue (Components|GetOwner))
  (Transformation|SetActorLocation _returnvalue (+ (Transformation|GetActorLocation _returnvalue) (* (Transformation|GetActorForwardVector _returnvalue) DeltaSeconds (Variables|Default|GetDirectionMultiplier))) false false))